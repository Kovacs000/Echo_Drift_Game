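; BP_CCTV is a security camera actor that films its view with a SceneCaptureComponent2D.
; On BeginPlay, a switch on CCTVID assigns the capture one of twelve fixed CCTV_Camera render targets, so each placed camera feeds its own texture.
; The construction script is empty, so the target is only set at runtime.
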(event EventBeginPlay
  (bind _scenecapturecomponent2d (Variables|Default|GetSceneCaptureComponent2D))
  ;[1 1 1] CamerasID
  (switch int (Variables|Default|GetCCTV%20ID)
    (:1
      (Variables|/Script/Engine.SceneCaptureComponent2D|SetTextureTarget _scenecapturecomponent2d "/Game/Cameras/CCTV_Camera_1.CCTV_Camera_1"))
    (:2
      (Variables|/Script/Engine.SceneCaptureComponent2D|SetTextureTarget _scenecapturecomponent2d "/Game/Cameras/CCTV_Camera_2.CCTV_Camera_2"))
    (:3
      (Variables|/Script/Engine.SceneCaptureComponent2D|SetTextureTarget _scenecapturecomponent2d "/Game/Cameras/CCTV_Camera_3.CCTV_Camera_3"))
    (:4
      (Variables|/Script/Engine.SceneCaptureComponent2D|SetTextureTarget _scenecapturecomponent2d "/Game/Cameras/CCTV_Camera_4.CCTV_Camera_4"))
    (:5
      (Variables|/Script/Engine.SceneCaptureComponent2D|SetTextureTarget _scenecapturecomponent2d "/Game/Cameras/CCTV_Camera_5.CCTV_Camera_5"))
    (:6
      (Variables|/Script/Engine.SceneCaptureComponent2D|SetTextureTarget _scenecapturecomponent2d "/Game/Cameras/CCTV_Camera_6.CCTV_Camera_6"))
    (:7
      (Variables|/Script/Engine.SceneCaptureComponent2D|SetTextureTarget _scenecapturecomponent2d "/Game/Cameras/CCTV_Camera_7.CCTV_Camera_7"))
    (:8
      (Variables|/Script/Engine.SceneCaptureComponent2D|SetTextureTarget _scenecapturecomponent2d "/Game/Cameras/CCTV_Camera_8.CCTV_Camera_8"))
    (:9
      (Variables|/Script/Engine.SceneCaptureComponent2D|SetTextureTarget _scenecapturecomponent2d "/Game/Cameras/CCTV_Camera_9.CCTV_Camera_9"))
    (:10
      (Variables|/Script/Engine.SceneCaptureComponent2D|SetTextureTarget _scenecapturecomponent2d "/Game/Cameras/CCTV_Camera_10.CCTV_Camera_10"))
    (:11
      (Variables|/Script/Engine.SceneCaptureComponent2D|SetTextureTarget _scenecapturecomponent2d "/Game/Cameras/CCTV_Camera_11.CCTV_Camera_11"))
    (:12
      (Variables|/Script/Engine.SceneCaptureComponent2D|SetTextureTarget _scenecapturecomponent2d "/Game/Cameras/CCTV_Camera_12.CCTV_Camera_12"))))

(fn ConstructionScript)